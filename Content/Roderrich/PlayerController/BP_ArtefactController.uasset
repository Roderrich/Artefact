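; BP_ArtefactController is a player controller that routes Enhanced Input actions to the player's third-person character.
; On BeginPlay it casts player character 0 to BP_ThirdPersonCharacter and caches the reference.
; Look, move, fire, jump and dash actions call matching functions on that character, with jump and dash also signalling release through their end functions.
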(event `self.ReceiveBeginPlay`
  (bind _asbp_third_person_character (cast `/Game/ThirdPerson/Blueprints/BP_ThirdPersonCharacter` (`GameplayStatics.GetPlayerCharacter` 0)))
  (set `self.As BP Third Person Character` _asbp_third_person_character))

(event `EnhancedInput|/Game/Roderrich/PlayerController/Inputs/IA_Looks`
  (params (ActionValue :type "Vector2D Structure") (ElapsedSeconds :type "Float (double-precision)") (TriggeredSeconds :type "Float (double-precision)") (InputAction :type "InputAction Object Reference" :default "/Game/Roderrich/PlayerController/Inputs/IA_Looks.IA_Looks"))
  (:`Triggered`
    (`/Game/ThirdPerson/Blueprints/BP_ThirdPersonCharacter.LookAround` (`self.As BP Third Person Character`) ActionValue_X ActionValue_Y)))

(event `EnhancedInput|/Game/Roderrich/PlayerController/Inputs/IA_Fire`
  (params (ActionValue :type Boolean) (ElapsedSeconds :type "Float (double-precision)") (TriggeredSeconds :type "Float (double-precision)") (InputAction :type "InputAction Object Reference" :default "/Game/Roderrich/PlayerController/Inputs/IA_Fire.IA_Fire"))
  (:`Triggered`
    (`/Game/ThirdPerson/Blueprints/BP_ThirdPersonCharacter.Fire` (`self.As BP Third Person Character`))))

(event `EnhancedInput|/Game/Roderrich/PlayerController/Inputs/IA_Moves`
  (params (ActionValue :type "Vector2D Structure") (ElapsedSeconds :type "Float (double-precision)") (TriggeredSeconds :type "Float (double-precision)") (InputAction :type "InputAction Object Reference" :default "/Game/Roderrich/PlayerController/Inputs/IA_Moves.IA_Moves"))
  (:`Triggered`
    (`/Game/ThirdPerson/Blueprints/BP_ThirdPersonCharacter.Move` (`self.As BP Third Person Character`) ActionValue_X ActionValue_Y)))

(event `EnhancedInput|/Game/Roderrich/PlayerController/Inputs/IA_Jumps`
  (params (ActionValue :type Boolean) (ElapsedSeconds :type "Float (double-precision)") (TriggeredSeconds :type "Float (double-precision)") (InputAction :type "InputAction Object Reference" :default "/Game/Roderrich/PlayerController/Inputs/IA_Jumps.IA_Jumps"))
  (bind _as_bp_third_person_character (`self.As BP Third Person Character`))
  (:`Triggered`
    (`/Game/ThirdPerson/Blueprints/BP_ThirdPersonCharacter.JumpStart` _as_bp_third_person_character))
  (:`Completed`
    (`/Game/ThirdPerson/Blueprints/BP_ThirdPersonCharacter.JumpEnd` _as_bp_third_person_character)))

(event `EnhancedInput|/Game/Roderrich/PlayerController/Inputs/IA_Dash`
  (params (ActionValue :type Boolean) (ElapsedSeconds :type "Float (double-precision)") (TriggeredSeconds :type "Float (double-precision)") (InputAction :type "InputAction Object Reference" :default "/Game/Roderrich/PlayerController/Inputs/IA_Dash.IA_Dash"))
  (bind _as_bp_third_person_character (`self.As BP Third Person Character`))
  (:`Triggered`
    (`/Game/ThirdPerson/Blueprints/BP_ThirdPersonCharacter.Dash` _as_bp_third_person_character))
  (:`Completed`
    (`/Game/ThirdPerson/Blueprints/BP_ThirdPersonCharacter.DashEnd` _as_bp_third_person_character)))

(fn `UserConstructionScript`)